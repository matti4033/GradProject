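; BP_Spider is a player-controlled spider character with Enhanced Input move and look controls.
; BeginPlay adds the default mapping context, caches the SpiderAnimInstance and stores the mesh's base relative transform.
; Each Tick, the body offsets from the anim instance drive the mesh: roll and pitch are added to the base rotation, while the height offset replaces relative Z in a swept move.
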(event `self.ReceiveTick`
  (params (DeltaSeconds :type "Float (single-precision)"))
  (bind _as_spider_anim_instance (`self.As Spider Anim Instance`))
  (`SceneComponent.K2_SetRelativeRotation` (`self.Mesh`) (`KismetMathLibrary.MakeRotator` (+ (.roll (`SpiderAnimInstance.BodyRotationOffset` _as_spider_anim_instance)) (.roll (`self.MeshBaseRotation`))) (+ (.pitch (`SpiderAnimInstance.BodyRotationOffset` _as_spider_anim_instance)) (.pitch (`self.MeshBaseRotation`))) (.yaw (`self.MeshBaseRotation`))) false false)
  (`SceneComponent.K2_SetRelativeLocation` (`self.Mesh`) (`KismetMathLibrary.MakeVector` (.x (`self.MeshBaseLocation`)) (.y (`self.MeshBaseLocation`)) (`SpiderAnimInstance.BodyHeightOffset` _as_spider_anim_instance)) true false))

(event `self.ReceiveBeginPlay`
  (bind _mesh (`self.Mesh`))
  (`EnhancedInputSubsystemInterface.AddMappingContext` (pcsubsystem `EnhancedInputLocalPlayerSubsystem` (`GameplayStatics.GetPlayerController` 0)) "/Game/ThirdPerson/Input/IMC_Default.IMC_Default" 0 (struct))
  (bind _asspider_anim_instance (cast `SpiderAnimInstance` (`SkeletalMeshComponent.GetAnimInstance` (`self.Mesh`))))
  (set `self.As Spider Anim Instance` _asspider_anim_instance)
  (set `self.MeshBaseRotation` (`SceneComponent.RelativeRotation` _mesh))
  (set `self.MeshBaseLocation` (`SceneComponent.RelativeLocation` _mesh)))

(event `EnhancedInput|/Game/ThirdPerson/Input/Actions/IA_Move`
  (params (ActionValue :type "Vector2D Structure") (ElapsedSeconds :type "Float (double-precision)") (TriggeredSeconds :type "Float (double-precision)") (InputAction :type "InputAction Object Reference" :default "/Game/ThirdPerson/Input/Actions/IA_Move.IA_Move"))
  (:`Triggered`
    (`self.AddMovementInput` (`self.GetActorForwardVector`) (.y (`KismetMathLibrary.Conv_Vector2DToVector` (`|GetInputActionValue`))))
    (`self.AddMovementInput` (`self.GetActorRightVector`) (.x (`KismetMathLibrary.Conv_Vector2DToVector` (`|GetInputActionValue`))))))

(event `EnhancedInput|/Game/ThirdPerson/Input/Actions/IA_Look`
  (params (ActionValue :type "Vector2D Structure") (ElapsedSeconds :type "Float (double-precision)") (TriggeredSeconds :type "Float (double-precision)") (InputAction :type "InputAction Object Reference" :default "/Game/ThirdPerson/Input/Actions/IA_Look.IA_Look"))
  (bind (_x _y) (`KismetMathLibrary.BreakVector2D` ActionValue))
  (:`Triggered`
    (`self.AddControllerYawInput` _x)
    (`self.AddControllerPitchInput` _y)))

(fn `UserConstructionScript`)