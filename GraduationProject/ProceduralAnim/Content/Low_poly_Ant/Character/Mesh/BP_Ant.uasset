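; BP_Ant is a player-controlled ant character with Enhanced Input movement and camera look.
; BeginPlay adds IMC_Default and caches a SpiderAnimInstance along with the mesh's base transform.
; IA_Move stores MovementInput and drives movement along the actor's forward and right vectors, while IA_Look feeds controller yaw and pitch.
; Logic applying the anim instance's body tilt and height offsets to the mesh exists but is disconnected, so it never runs.
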(event `self.ReceiveTick`
  (params (DeltaSeconds :type "Float (single-precision)")))

(event `self.ReceiveBeginPlay`
  (bind _mesh (`self.Mesh`))
  (`EnhancedInputSubsystemInterface.AddMappingContext` (pcsubsystem `EnhancedInputLocalPlayerSubsystem` (`GameplayStatics.GetPlayerController` 0)) "/Game/ThirdPerson/Input/IMC_Default.IMC_Default" 0 (struct))
  (bind _asspider_anim_instance (cast `SpiderAnimInstance` (`SkeletalMeshComponent.GetAnimInstance` (`self.Mesh`))))
  (set `self.As Spider Anim Instance` _asspider_anim_instance)
  (set `self.MeshBaseRotation` (`SceneComponent.RelativeRotation` _mesh))
  (set `self.MeshBaseLocation` (`SceneComponent.RelativeLocation` _mesh)))

(event `EnhancedInput|/Game/ThirdPerson/Input/Actions/IA_Move`
  (params (ActionValue :type "Vector2D Structure") (ElapsedSeconds :type "Float (double-precision)") (TriggeredSeconds :type "Float (double-precision)") (InputAction :type "InputAction Object Reference" :default "/Game/ThirdPerson/Input/Actions/IA_Move.IA_Move"))
  (bind (_x _y) (`KismetMathLibrary.BreakVector2D` ActionValue))
  (:`Triggered`
    (set `self.MovementInput` (`KismetMathLibrary.MakeVector2D` _y _x))
    (`self.AddMovementInput` (`self.GetActorForwardVector`) (.y (`KismetMathLibrary.Conv_Vector2DToVector` (`|GetInputActionValue`))))
    (`self.AddMovementInput` (`self.GetActorRightVector`) (.x (`KismetMathLibrary.Conv_Vector2DToVector` (`|GetInputActionValue`)))))
  (:`Completed`
    (set `self.MovementInput` (0.0 0.0))))

(event `EnhancedInput|/Game/ThirdPerson/Input/Actions/IA_Look`
  (params (ActionValue :type "Vector2D Structure") (ElapsedSeconds :type "Float (double-precision)") (TriggeredSeconds :type "Float (double-precision)") (InputAction :type "InputAction Object Reference" :default "/Game/ThirdPerson/Input/Actions/IA_Look.IA_Look"))
  (bind (_x _y) (`KismetMathLibrary.BreakVector2D` ActionValue))
  (:`Triggered`
    (`self.AddControllerYawInput` _x)
    (`self.AddControllerPitchInput` _y)))

(fn `UserConstructionScript`)